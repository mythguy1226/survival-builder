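; Player character for a grid-based building game, handling camera-style movement, building placement and the build, upgrade and pause widgets.
; Choosing a building starts a delayed loop that traces under the cursor and snaps a preview actor to BP_GridManager cells.
; Left click places the preview, with walls painted cell by cell on Tick while held; right click cancels.
; Left click without a preview opens an upgrade widget, and Tab toggles the pause widget.
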(event Custom|OnBuildButtonClicked
  (params (BuildingClass :type BP%20Build%20Actor%20Class%20Reference))
  (bind _output_get (Variables|Default|SetCurrentlySelectedBuilding BuildingClass))
  (Variables|Default|SetPlacing true)
  (CallFunction|TryPlace _output_get :!label _label)
  (Utilities|FlowControl|Delay 0.01)
  (goto _label))

(event Input|EnhancedActionEvents|EnhancedInputActionIA_Move_Vertical
  (params (ActionValue :type Float%20%28double-precision%29) (ElapsedSeconds :type Float%20%28double-precision%29) (TriggeredSeconds :type Float%20%28double-precision%29) (InputAction :type Input%20Action%20Object%20Reference :default "/Game/Maps/Input/Inputs/IA_Move_Vertical.IA_Move_Vertical"))
  (:Triggered
    (Transformation|AddActorWorldOffset (* (Class|KismetMathLibrary|VectorRight) ActionValue (Variables|Default|GetMoveSpeed)))))

(event Input|EnhancedActionEvents|EnhancedInputActionIA_Move_Horizontal
  (params (ActionValue :type Float%20%28double-precision%29) (ElapsedSeconds :type Float%20%28double-precision%29) (TriggeredSeconds :type Float%20%28double-precision%29) (InputAction :type Input%20Action%20Object%20Reference :default "/Game/Maps/Input/Inputs/IA_Move_Horizontal.IA_Move_Horizontal"))
  (:Triggered
    (Transformation|AddActorWorldOffset (* ActionValue (Class|KismetMathLibrary|VectorForward) (Variables|Default|GetMoveSpeed)))))

(event EventBeginPlay
  (bind _asplayer_controller (Utilities|Casting|CastToPlayerController (Pawn|GetController)))
  (Input|AddMappingContext (PlayerController|LocalPlayerSubsystems|GetEnhancedInputLocalPlayerSubsystem _asplayer_controller) "/Game/Maps/Input/InputMappingContext.InputMappingContext" 0 "(bIgnoreAllPressedKeysUntilRelease=True,bForceImmediately=False)")
  (bind _returnvalue (Actor|GetActorOfClass "/Game/Blueprints/BP_GridManager.BP_GridManager_C"))
  (Variables|Default|SetBP_GridManager _returnvalue)
  (bind _returnvalue_2 (UserInterface|CreateWidget "/Game/Maps/UI/BP_PlayerUI.BP_PlayerUI_C" (Game|GetPlayerController 0)))
  (UserInterface|Viewport|AddtoViewport _returnvalue_2 0))

(event EventTick
  (params (DeltaSeconds :type Float%20%28single-precision%29))
  (if (Variables|Default|GetbIsConstructingWall)
    (CallFunction|ConstructWall)))

(event Input|MouseEvents|LeftMouseButton
  (params (Key :type Key%20Structure :default "None"))
  (bind _returnvalue (Game|GetPlayerController 0))
  (bind (_worldlocation _worlddirection) (Game|Player|ConvertMouseLocationToWorldSpace _returnvalue))
  (:Pressed
    (Utilities|IsValid (Variables|Default|GetSpawnActor)
      (:Is%20Valid
        (if (Utilities|IsValidClass (Variables|Default|GetCurrentlySelectedBuilding))
          (if (!= (Variables|Default|GetCurrentlySelectedBuilding) "/Game/Maps/Blueprints/Wall.Wall_C")
            _
            (else
              (Variables|Default|SetbIsConstructingWall true)))
          (bind _bsuccessfulplaced (Default|Place (Variables|Default|GetSpawnActor)))
          (if _bsuccessfulplaced
            (Variables|Default|SetPlacing false)
            (Variables|Default|SetCurrentlySelectedBuilding 0)
            (Variables|Default|SetSpawnActor 0)
            (if (Variables|Default|GetisLumerMill)
              _))))
      (:Is%20Not%20Valid
        (bind _outhit (Collision|LineTraceForObjects _worldlocation (+ _worldlocation (* _worlddirection 4e+03)) (Variables|Default|GetObject%20Types) false 0 "None"))
        (bind _returnvalue_2 (UserInterface|CreateWidget "/Game/Maps/UI/WI_Upgrade.WI_Upgrade_C"))
        (UserInterface|Viewport|AddtoViewport _returnvalue_2 0))))
  (:Released
    (Variables|Default|SetbIsConstructingWall false)))

(event Input|KeyboardEvents|Tab
  (params (Key :type Key%20Structure :default "None"))
  (:Pressed
    (Utilities|FlowControl|FlipFlop
      (:A
        (bind _returnvalue (UserInterface|CreateWidget "/Game/Maps/UI/W_Pause.W_Pause_C"))
        (UserInterface|Viewport|AddtoViewport _returnvalue 0)
        (Widget|SetVisibility _returnvalue "Visible"))
      (:B
        (Widget|RemovefromParent _returnvalue)))))

(event Input|MouseEvents|RightMouseButton
  (params (Key :type Key%20Structure :default "None"))
  (bind _spawnactor (Variables|Default|GetSpawnActor))
  (:Pressed
    (Variables|Default|SetCurrentlySelectedBuilding 0)
    (Utilities|IsValid _spawnactor
      (:Is%20Valid
        (Actor|DestroyActor _spawnactor)
        (Variables|Default|SetisLumerMill false)
        (Variables|Default|SetbIsConstructingWall false)
        (Variables|Default|SetPlacing false)))))

(fn ConstructionScript)

(fn TryPlace
  (params (Actor :type BP%20Build%20Actor%20Class%20Reference))
  (bind _returnvalue (Game|GetPlayerController 0))
  (bind _bp_gridmanager (Variables|Default|GetBP_GridManager))
  (bind (_worldlocation _worlddirection) (Game|Player|ConvertMouseLocationToWorldSpace _returnvalue))
  (if (Variables|Default|GetPlacing)
    (bind _outactors (Actor|GetAllActorsOfClass "/Game/Maps/Blueprints/BP_BuildActor.BP_BuildActor_C"))
    (bind (_outhit _returnvalue_2) (Collision|LineTraceByChannel _worldlocation (+ _worldlocation (* _worlddirection (Variables|Default|GetTraceDistance))) "TraceTypeQuery1" false _outactors "None"))
    (if _returnvalue_2
      (Utilities|IsValid _bp_gridmanager
        (:Is%20Valid
          (bind _returnvalue_3 (Class|GridManager|GetCellPosfromWorldPos _bp_gridmanager (.Location (Collision|BreakHitResult _outhit))))
          (Variables|Default|SetCurrLoc _returnvalue_3)
          (Utilities|IsValid (Variables|Default|GetSpawnActor)
            (:Is%20Valid
              (Transformation|SetActorLocation (Variables|Default|GetSpawnActor) _returnvalue_3 false false)
              (Default|CheckSpawn (Variables|Default|GetSpawnActor)))
            (:Is%20Not%20Valid
              (bind _returnvalue_4 (Game|SpawnActorfromClass Actor (Math|Transform|MakeTransform _returnvalue_3 "0, 0, 0" "1.000000,1.000000,1.000000") "Undefined" "MultiplyWithRoot" 0 0))
              (bind _output_get (Variables|Default|SetSpawnActor _returnvalue_4))
              (Variables|/Game/Maps/Blueprints/BP_BuildActor.BP_BuildActor_C|SetMaterial _output_get (Rendering|Material|GetMaterial (Variables|/Game/Maps/Blueprints/BP_BuildActor.BP_BuildActor_C|GetMesh _output_get) 0))
              (Default|CheckSpawn _output_get)))))
      (else
        (Utilities|IsValid (Variables|Default|GetSpawnActor)
          (:Is%20Valid
            (Actor|DestroyActor (Variables|Default|GetSpawnActor))))))))

(fn AddSlottoInventory
  (bind _outrownames (DataTable|GetDataTableRowNames "/Game/Maps/Inventory/DT_Slot.DT_Slot"))
  (for _array_element _outrownames
    (Variables|Default|SetNameOfRow (Utilities|String|ToString(Name) _array_element))))

(fn ConstructWall
  (bind _returnvalue (Game|GetPlayerController 0))
  (bind _bp_gridmanager (Variables|Default|GetBP_GridManager))
  (bind (_worldlocation _worlddirection) (Game|Player|ConvertMouseLocationToWorldSpace _returnvalue))
  (bind _outactors (Actor|GetAllActorsOfClass "/Game/Maps/Blueprints/BP_BuildActor.BP_BuildActor_C"))
  (bind (_outhit _returnvalue_2) (Collision|LineTraceByChannel _worldlocation (+ _worldlocation (* _worlddirection (Variables|Default|GetTraceDistance))) "TraceTypeQuery1" false _outactors "None"))
  (if _returnvalue_2
    (Utilities|IsValid _bp_gridmanager
      (:Is%20Valid
        (bind _returnvalue_3 (Class|GridManager|IsCellEmpty _bp_gridmanager (.Location (Collision|BreakHitResult _outhit))))
        (if _returnvalue_3
          (bind _returnvalue_4 (Class|GridManager|GetCellPosfromWorldPos _bp_gridmanager (.Location (Collision|BreakHitResult _outhit))))
          (bind _returnvalue_5 (Game|SpawnActorfromClass "/Game/Maps/Blueprints/Wall.Wall_C" (Math|Transform|MakeTransform _returnvalue_4 "0, 0, 0" "1.000000,1.000000,1.000000") "Undefined" "MultiplyWithRoot" 0 0))
          (Variables|/Game/Maps/Blueprints/BP_BuildActor.BP_BuildActor_C|SetMaterial _returnvalue_5 "/Game/StarterContent/Materials/M_Wood_Floor_Walnut_Polished.M_Wood_Floor_Walnut_Polished")
          (Variables|/Game/Maps/Blueprints/BP_BuildActor.BP_BuildActor_C|SetCanSpawn _returnvalue_5 true)
          (Default|Place _returnvalue_5))))))