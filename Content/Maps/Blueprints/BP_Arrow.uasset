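; BP_Arrow is a projectile actor that damages werewolves on contact.
; Its Box overlap finds a BP_CombatComponent on the other actor, requires it to be a BP_Werewolf, applies ProjectileDamage credited to ShotOwner, then destroys the arrow a tick later.
; A Tick countdown from Lifetime destroys arrows that outlive their timer.
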(event OnComponentBeginOverlap(Box)
  (params (OverlappedComponent :type Primitive%20Component%20Object%20Reference) (OtherActor :type Actor%20Object%20Reference) (OtherComp :type Primitive%20Component%20Object%20Reference) (OtherBodyIndex :type Integer) (bFromSweep :type Boolean) (SweepResult :type Hit%20Result%20Structure%20%28by%20ref%29))
  (bind _returnvalue (Actor|GetComponentbyClass OtherActor "/Game/Blueprints/AI/Components/BP_CombatComponent.BP_CombatComponent_C"))
  ;[1 1 1] Handle collisions with arrow
  (Utilities|IsValid _returnvalue
    (:Is%20Valid
      (Utilities|Casting|CastToBP_Werewolf OtherActor)
      (Default|TakeDamage _returnvalue (Variables|Default|GetProjectileDamage) (Variables|Default|GetShotOwner))
      (Utilities|FlowControl|DelayUntilNextTick)
      (Actor|DestroyActor))))

(event EventBeginPlay
  (Variables|Default|SetLifeTimer (Variables|Default|GetLifetime)))

(event Collision|EventActorBeginOverlap
  (params (OtherActor :type Actor%20Object%20Reference)))

(event EventTick
  (params (DeltaSeconds :type Float%20%28single-precision%29))
  ;[1 1 1] Arrows will be destroyed after their lifetime is up
  (Variables|Default|SetLifeTimer (- (Variables|Default|GetLifeTimer) DeltaSeconds))
  (if (<= (Variables|Default|GetLifeTimer) 0.0)
    (Actor|DestroyActor)))

(fn ConstructionScript)