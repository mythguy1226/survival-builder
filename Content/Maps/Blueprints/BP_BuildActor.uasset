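; BP_BuildActor is a placeable building that previews where it can go and costs wood to build.
; CheckSpawn asks BP_GridManager whether its cell is empty and tints the mesh green or red.
; Place charges the player's resource component, then restores the material, enables blocking collision and marks the cell occupied, or destroys the actor if payment fails.
; Its health bar widget turns about the vertical axis to face the camera each tick.
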(event EventTick
  (params (DeltaSeconds :type Float%20%28single-precision%29))
  (bind _returnvalue (Game|GetPlayerCameraManager 0))
  (bind _widget (Variables|Default|GetWidget))
  (bind _returnvalue_2 (Camera|GetCameraLocation _returnvalue))
  (bind _returnvalue_3 (Transformation|GetWorldLocation _widget))
  (Transformation|SetWorldRotation (Variables|Default|GetWidget) (Math|Vector|RotatorfromAxisandAngle "0.000000,0.000000,1.000000" (Class|KismetMathLibrary|DegAtan2 (- (.y _returnvalue_2) (.y _returnvalue_3)) (- (.x _returnvalue_2) (.x _returnvalue_3)))) false false))

(event EventBeginPlay
  (bind _returnvalue (Actor|GetActorOfClass "/Game/Blueprints/BP_GridManager.BP_GridManager_C"))
  (Variables|Default|SetBP_GridManager _returnvalue)
  (bind _asbp_character (Utilities|Casting|CastToBP_Character (Game|GetPlayerCharacter 0)))
  (Variables|Default|SetBP_PlayerCharacter _asbp_character)
  ;[1 1 1] Initialize owning actor of health bar widget to be this actor
  (bind _asbp_healthbar (Utilities|Casting|CastToBP_Healthbar (UserInterface|GetWidget (Variables|Default|GetWidget))))
  (Variables|/Game/Blueprints/AI/BP_Healthbar.BP_Healthbar_C|SetOwningActor _asbp_healthbar (Components|GetOwner (Variables|Default|GetMesh))))

(fn ConstructionScript)

(fn CheckSpawn
  (bind _mesh (Variables|Default|GetMesh))
  (bind _bp_gridmanager (Variables|Default|GetBP_GridManager))
  (Utilities|IsValid _bp_gridmanager
    (:Is%20Valid
      (bind _returnvalue (Class|GridManager|IsCellEmpty _bp_gridmanager (Transformation|GetActorLocation)))
      (if (not _returnvalue)
        (Rendering|Material|SetMaterial _mesh 0 "/Game/Maps/Materials/M_Red.M_Red")
        (Variables|Default|SetCanSpawn false)
        (else
          (Rendering|Material|SetMaterial _mesh 0 "/Game/Maps/Materials/M_Green.M_Green")
          (Variables|Default|SetCanSpawn true))))))

(fn Place
  (bind _mesh (Variables|Default|GetMesh))
  (if (Variables|Default|GetCanSpawn)
    (bind _canbuild (Default|WoodCollection (Variables|/Game/Maps/Blueprints/BP_Character.BP_Character_C|GetBP_ResourceComponent (Variables|Default|GetBP_PlayerCharacter)) (Variables|Default|GetWoodCost)))
    (if _canbuild
      (Rendering|Material|SetMaterial _mesh 0 (Variables|Default|GetMaterial))
      (Collision|SetCollisionProfileName _mesh "BlockAllDynamic" true :!class /Script/Engine.PrimitiveComponent)
      (Class|GridManager|SetIsCellEmpty (Variables|Default|GetBP_GridManager) (Transformation|GetActorLocation) false)
      (return true)
      (else
        (Actor|DestroyActor))))
  (return false))