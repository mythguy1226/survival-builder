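; Combat component shared by AI units and buildings, handling health, damage, melee hit checks and cooldown-gated projectile firing.
; GenerateHitSphere sphere-traces and damages the hit actor's combat component unless it shares the owner's class.
; TakeDamage handles death per owner: werewolves reset and clear outpost targeting, town hall loss opens game over, other buildings free their grid cell and are destroyed.
; LaunchProjectile spawns projectiles, tagging arrows with their shooter, while Tick restores firing.
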(event EventBeginPlay
  (Variables|Default|SetHealth (Variables|Default|GetMaxHealth)))

(event EventTick
  (params (DeltaSeconds :type Float%20%28single-precision%29))
  (if (not (Variables|Default|GetCanShoot))
    (Variables|Default|SetProjectileTimer (- (Variables|Default|GetProjectileTimer) DeltaSeconds))
    (if (<= (Variables|Default|GetProjectileTimer) 0.0)
      (Variables|Default|SetCanShoot true)
      (Variables|Default|SetProjectileTimer (Variables|Default|GetProjectileCooldown)))))

(fn GetHealth
  ;[1 1 1] Health Getter
  (return (Variables|Default|GetHealth)))

(fn TakeDamage
  (params (Damage :type Float%20%28double-precision%29) (Damager%20Actor :type Actor%20Object%20Reference))
  (bind _returnvalue (Components|GetOwner))
  ;[1 1 1] Negate health and handle death
  (Variables|Default|SetHealth (- (CallFunction|GetHealth) Damage))
  (if (<= (CallFunction|GetHealth) 0.0)
    (bind _asbp_werewolf (Utilities|Casting|CastToBP_Werewolf _returnvalue)
      (:then
        (Default|ResetEnemy _asbp_werewolf)
        ;[1 1 1] Reset target detection if tower killed their enemy
        (Utilities|IsValid Damager%20Actor
          (:Is%20Valid
            (bind _outactors (Actor|GetAllActorsOfClass "/Game/Blueprints/AI/Controllers/BP_OutpostController.BP_OutpostController_C"))
            (for _array_element _outactors
              (Default|ClearTargetDetection _array_element)))))
      (:CastFailed
        (Utilities|Casting|CastToBP_TownHall _returnvalue
          (:then
            (Game|OpenLevel(byName) "GameOverScene"))
          (:CastFailed
            (bind _asbp_build_actor (Utilities|Casting|CastToBP_BuildActor _returnvalue))
            (Class|GridManager|SetIsCellEmpty (Variables|/Game/Maps/Blueprints/BP_BuildActor.BP_BuildActor_C|GetBP_GridManager _asbp_build_actor) (Transformation|GetActorLocation _asbp_build_actor) true)
            (Actor|DestroyActor _returnvalue)))))))

(fn GenerateHitSphere
  (params (Location :type Vector) (Radius :type Float%20%28double-precision%29) (Damage :type Float%20%28double-precision%29) (Debug%20Mode :type Boolean))
  ;[1 1 1] Generate the sphere trace to check for attack collisions
  (LocalVariables|SetAttackDamage Damage)
  (if Debug%20Mode
    (LocalVariables|SetDebugType "ForDuration")
    (else
      (LocalVariables|SetDebugType "None")))
  (bind (_outhit _returnvalue) (Collision|SphereTraceByChannel Location Location Radius "TraceTypeQuery1" false 0 (LocalVariables|GetDebugType)))
  ;[1 1 1] If something damageable was hit then call upon its combat component to deal damage
  (if _returnvalue
    (Utilities|IsValid (Actor|GetComponentbyClass (.HitActor (Collision|BreakHitResult _outhit)) "BP_CombatComponent_C")
      (:Is%20Valid
        (if (!= (Utilities|GetClass (Components|GetOwner)) (Utilities|GetClass (.HitActor (Collision|BreakHitResult _outhit))))
          (CallFunction|TakeDamage (Actor|GetComponentbyClass (.HitActor (Collision|BreakHitResult _outhit)) "BP_CombatComponent_C") (LocalVariables|GetAttackDamage)))))))

(fn LaunchProjectile
  (params (Projectile%20Class :type Actor%20Class%20Reference) (Launch%20Transform :type Transform))
  (bind _returnvalue (Components|GetOwner))
  ;[1 1 1] Launch projectile and update shoot status
  (if (Variables|Default|GetCanShoot)
    (bind _returnvalue_2 (Game|SpawnActorfromClass Projectile%20Class Launch%20Transform "AlwaysSpawn" "MultiplyWithRoot" 0 0))
    (Variables|Default|SetCanShoot false)
    (bind _asbp_arrow (Utilities|Casting|CastToBP_Arrow _returnvalue_2))
    (Utilities|IsValid _returnvalue
      (:Is%20Valid
        (Variables|/Game/Maps/Blueprints/BP_Arrow.BP_Arrow_C|SetShotOwner _asbp_arrow _returnvalue)))))